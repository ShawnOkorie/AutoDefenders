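; BP_EnemyManager is an enemy spawner that creates a batch of BP_Enemy actors shortly after play begins.
; BeginPlay waits briefly, caches the BP_PlayerBase actor, then calls SpawnEnemy in a fixed loop.
; SpawnEnemy offsets spawns by SpawnDistance at random yaw around world origin, passing in the base.
; Spawn rotation looks toward the base from the origin at random height, and SpawnWave is an empty stub.
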(event EventBeginPlay
  (Utilities|FlowControl|Delay 0.1)
  (bind _returnvalue (Actor|GetActorOfClass "/Game/Blueprints/BP_PlayerBase.BP_PlayerBase_C"))
  (Variables|Default|SetPlayerBase _returnvalue)
  (for _index (range 0 20)
    (CallFunction|SpawnEnemy)))

(event Collision|EventActorBeginOverlap
  (params (OtherActor :type Actor%20Object%20Reference)))

(event EventTick
  (params (DeltaSeconds :type Float%20%28single-precision%29)))

(fn ConstructionScript)

(fn SpawnEnemy
  (bind _returnvalue (Class|KismetMathLibrary|VectorForward))
  (bind _returnvalue_2 (Math|Random|RandomFloatinRange 0.0 3.6e+02))
  (bind _playerbase (Variables|Default|GetPlayerBase))
  (bind _spawndistance (Variables|Default|GetSpawnDistance))
  (bind _returnvalue_3 (* _returnvalue _spawndistance))
  (bind _returnvalue_4 (Math|Vector|RotateVector _returnvalue_3 (Math|Rotator|MakeRotator 0.0 0.0 _returnvalue_2)))
  (Utilities|IsValid _playerbase
    (:Is%20Valid
      (Game|SpawnActorfromClass "/Game/Blueprints/BP_Enemy.BP_Enemy_C" (Math|Transform|MakeTransform (Math|Vector|MakeVector (.x _returnvalue_4) (.y _returnvalue_4) 8e+01) (Math|Rotator|FindLookatRotation (Math|Vector|MakeVector 0.0 0.0 _returnvalue_2) (Transformation|GetActorLocation (Variables|Default|GetPlayerBase))) "1.000000,1.000000,1.000000") "Undefined" "MultiplyWithRoot" 0 _playerbase 0))))

(fn SpawnWave)